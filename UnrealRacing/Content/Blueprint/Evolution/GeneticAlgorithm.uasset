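; Genetic algorithm manager that holds a population of GenomeData objects and tracks their evaluation from one generation to the next.
; It hands out Ready genomes for evaluation and reports when all are Done.
; Selection only sorts and prints the population, and mutation just flags the first 90% of the array, with no crossover here.
; Separate helpers reset fitness and state and advance the generation counter.
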(event Custom|InitializePopulation
  (for _index (range 1 (Variables|Default|GetPopulationSize))
    (bind _returnvalue (Game|ConstructObjectfromClass "/Script/UnrealRacing.GenomeData" self))
    (bind _returnvalue_2 (Utilities|Array|Add (Variables|Default|GetPopulation) _returnvalue))
    (Variables|/Script/UnrealRacing.GenomeData|SetgenomeID _returnvalue _returnvalue_2)))

(fn GetNextGenomeforEvaluation
  (for _array_element (Variables|Default|GetPopulation)
    (if (Utilities|Enum|Equal(Enum) (Variables|/Script/UnrealRacing.GenomeData|GetevaluationState _array_element) "Ready")
      (Variables|/Script/UnrealRacing.GenomeData|SetevaluationState _array_element "Evaluating")
      (return true _array_element)))
  (return false 0))

(fn PrintPopulation
  (for _array_element (Variables|Default|GetPopulation)
    (Development|PrintString 0 (Utilities|String|Append (Utilities|GetObjectName _array_element) "/" (Utilities|String|ToString(Integer) (Variables|/Script/UnrealRacing.GenomeData|GetgenomeID _array_element)) "/" (Utilities|String|ToString(Float) (Variables|/Script/UnrealRacing.GenomeData|Getfitness _array_element))))))

(fn IsGenerationCompletelySimulated
  (for _array_element (Variables|Default|GetPopulation)
    (if (not (Utilities|Enum|Equal(Enum) (Variables|/Script/UnrealRacing.GenomeData|GetevaluationState _array_element) "Done"))
      (return false)))
  (return true))

(fn MutatePopulation
  (for (_array_element _array_index) (Variables|Default|GetPopulation)
    (if (< _array_index (Math|Float|Truncate (* (Variables|Default|GetPopulationSize) 0.9)))
      (Variables|/Script/UnrealRacing.GenomeData|SetshouldMutate _array_element true))))

(fn Selection
  (bind _sortedarray (Class|EvaluationFunctionLibrary|SortPopulation (Variables|Default|GetPopulation)))
  (Variables|Default|SetPopulation _sortedarray)
  (CallFunction|PrintPopulation))

(fn SetStatetoReadyandResetFitness
  (for _array_element (Variables|Default|GetPopulation)
    (Utilities|FlowControl|Sequence
      (:then_0
        (Variables|/Script/UnrealRacing.GenomeData|Setfitness _array_element 0.0))
      (:then_1
        (Variables|/Script/UnrealRacing.GenomeData|SetevaluationState _array_element "Ready")))))

(fn IncrementGenerationNumber
  (bind _result (Math|Integer|IncrementInt (Variables|Default|GetGeneration))
    (:%20%20
      (Development|PrintString 0 (Utilities|String|Append "Next Generation: " (Utilities|String|ToString(Integer) _result))))))