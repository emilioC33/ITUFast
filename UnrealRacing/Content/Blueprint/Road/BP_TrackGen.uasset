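; BP_TrackGen is an unfinished procedural track generator that runs SpawnTrack on BeginPlay.
; It computes points along an arc of radius 100 with degree-based sine and cosine, but the step storing them in TrackPoints is disconnected.
; It then spawns a BP_Track at an unset transform and clears its RoadDataArray.
; The final loop over TrackPoints is empty, so no road data gets filled in.
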(event EventBeginPlay
  (CallFunction|SpawnTrack))

(event Collision|EventActorBeginOverlap
  (params (OtherActor :type Actor%20Object%20Reference)))

(event EventTick
  (params (DeltaSeconds :type Float%20%28single-precision%29)))

(fn ConstructionScript)

(fn GenerateRandomPointinRadius
  (params (x :type Float%20%28single-precision%29) (Shape :type String))
  (LocalVariables|SetLocal_x x)
  (if (Utilities|Enum|Equal(Enum) Shape "Circle")
    (bind _output_get (LocalVariables|SetLocal_transform (Math|Vector2D|MakeVector2D (* (Math|Trig|Cos(Degrees) (LocalVariables|GetLocal_x)) 1e+02) (* (Math|Trig|Sin(Degrees) (LocalVariables|GetLocal_x)) 1e+02))))))

(fn SpawnTrack
  (for _index (range 0 11)
    (CallFunction|GenerateRandomPointinRadius (* _index 1e+01) "Circle"))
  (bind _output_get (LocalVariables|SetLocal_SpawnPoint ""))
  (bind _returnvalue (Game|SpawnActorfromClass "/Game/Blueprint/Road/BP_Track.BP_Track_C" _output_get "Undefined" 0 0))
  (Utilities|Array|Clear (Variables|/Game/Blueprint/Road/BP_Track.BP_Track_C|GetRoadDataArray _returnvalue))
  (for _index_2 (range 0 (- (Utilities|Array|Length (Variables|Default|GetTrackPoints)) 1))
    _))