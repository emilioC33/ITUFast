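; HumanPC is the human player's controller for driving a Sedan car pawn.
; On BeginPlay it caches the possessed Sedan, then forwards steering, throttle, handbrake and camera-switch input to it.
; A PrintFitness helper, not called in this file, prints the car's normalized progress along the track spline, divided by evaluation time relative to maximum track time.
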(event EventBeginPlay
  (bind _assedan (Utilities|Casting|CastToSedan (Pawn|GetControlledPawn)))
  (Variables|Default|SetCarPawn _assedan))

(event EventTick
  (params (DeltaSeconds :type Float%20%28single-precision%29)))

(event Input|ActionEvents|InputActionSwitchCamera
  (params (Key :type Key%20Structure))
  ;[1 1 1] Switch Camera
  (:Pressed
    (Default|SwitchCamera (Variables|Default|GetCarPawn))))

(event Input|ActionEvents|InputActionHandbrake
  (params (Key :type Key%20Structure))
  (bind _carpawn (Variables|Default|GetCarPawn))
  ;[1 1 1] Handbreak
  (:Pressed
    (Default|Handbreak _carpawn true))
  (:Released
    (Default|Handbreak _carpawn false)))

(event Input|AxisEvents|InputAxisMoveForward
  (params (AxisValue :type Float%20%28single-precision%29))
  ;[1 1 1] Throttle
  (Default|Throttle (Variables|Default|GetCarPawn) AxisValue))

(event Input|AxisEvents|InputAxisMoveRight
  (params (AxisValue :type Float%20%28single-precision%29))
  ;[1 1 1] Steer
  (Default|Steer (Variables|Default|GetCarPawn) AxisValue))

(fn ConstructionScript)

(fn PrintFitness
  (bind _trackref (Variables|Default|GetTrackRef))
  (Development|PrintString (Utilities|String|Append "Distance: " (Utilities|String|ToString(Float) (/ (CallFunction|FindDistanceAlongSpline (Transformation|GetActorLocation (Variables|Default|GetCarPawn)) (Variables|/Game/Blueprint/Road/BP_Track.BP_Track_C|GetSpline _trackref)) (/ (Variables|Default|GetevaluationTime) (Default|CalculateMaxTrackTime _trackref)))))))

(fn FindDistanceAlongSpline
  (params (Location :type Vector) (Spline :type Spline%20Component%20Object%20Reference))
  (return (/ (Class|SplineComponent|FindInputKeyClosesttoWorldLocation Spline Location) (Math|Conversions|ToFloat(Integer) (- (Spline|GetNumberOfSplinePoints Spline) (Math|Conversions|ToInteger(Boolean) (not (Class|SplineComponent|IsClosedLoop Spline))))))))