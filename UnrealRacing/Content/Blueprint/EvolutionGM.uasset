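; Game mode that evolves self-driving Sedans with a genetic algorithm, scoring genomes on BP_Track spline tracks flagged for evaluation.
; BeginPlay initializes the population, picks a random track and spawns a pool of AI cars that ignore each other.
; Idle cars are teleported to the track start, and their TensorflowController evaluates the next genome.
; Once all finish, it writes fitness, runs selection and mutation, and picks a random track for the next generation.
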(event EventBeginPlay
  (Utilities|FlowControl|Sequence
    (:then_0
      ;[1 1 1] Construct the Genetic Algorithm and Initialize a population
      (bind _returnvalue (Game|ConstructObjectfromClass "/Game/Blueprint/Evolution/GeneticAlgorithm.GeneticAlgorithm_C" self))
      (bind _output_get (Variables|Evolution|SetGeneticAlgorithm _returnvalue))
      (Default|InitializePopulation _output_get))
    (:then_1
      ;[1 1 1] Find Tracks
      (Utilities|FlowControl|Sequence
        (:then_0
          (bind _outactors (Actor|GetAllActorsOfClass "/Game/Blueprint/Road/BP_Track.BP_Track_C"))
          (for _array_element _outactors
            (if (Variables|/Game/Blueprint/Road/BP_Track.BP_Track_C|GetUseInEvaluation _array_element)
              (Utilities|Array|Add (Variables|Evolution|GetTracks) _array_element))))
        (:then_1
          (CallFunction|SelectRandomTrack))))
    (:then_2
      ;[1 1 1] Spawn Evaluators
      (for _index (range 1 (Variables|Evolution|GetNumberOfEvaluators))
        (bind _returnvalue_2 (AI|SpawnAIFromClass "/Game/Blueprint/Sedan/Sedan.Sedan_C" 0 "100000.000000, 0,100.000000" "0, 0, 0" true))
        (bind _assedan (Utilities|Casting|CastToSedan _returnvalue_2))
        (Utilities|Array|Add (Variables|Evolution|GetCars) _assedan))
      (CallFunction|IgnoreOtherEvaluators))
    (:then_3
      ;[1 1 1] Start Evolution
      (for _array_element_2 (Variables|Evolution|GetCars)
        (CallFunction|TryEvaluateNextGenome _array_element_2)))))

(event EventTick
  (params (DeltaSeconds :type Float%20%28single-precision%29)))

(fn ConstructionScript)

(fn GetSpawnatTrack
  (params (Track :type Integer))
  (bind _tracks (Variables|Evolution|GetTracks))
  (bind _output (Utilities|Array|Get(acopy) _tracks Track))
  (bind _spline (Variables|/Game/Blueprint/Road/BP_Track.BP_Track_C|GetSpline _output))
  (return (Spline|GetLocationatSplinePoint _spline 0 "World") (Spline|GetRotationatSplinePoint _spline 0 "Local")))

(fn TeleportCartoStartOfTrack
  (params (Car :type Sedan%20Object%20Reference) (TrackNumber :type Integer))
  (Utilities|FlowControl|Sequence
    (:then_0
      ;[1 1 1] Stop movement
      (Components|Movement|StopMovementImmediately (Variables|/Script/PhysXVehicles.WheeledVehicle|GetVehicleMovement Car)))
    (:then_1
      ;[1 1 1] Move Actor to new Spawn on track
      (bind (_spawnpointlocation _spawnpointrotation) (CallFunction|GetSpawnatTrack TrackNumber))
      (Utilities|FlowControl|Sequence
        (:then_0
          (Transformation|SetActorLocation Car (+ (LocalVariables|GetSpawnOffset) _spawnpointlocation) false true))
        (:then_1
          (Transformation|SetActorRotation Car _spawnpointrotation true))))
    (:then_2
      ;[1 1 1] Return the current track
      (return (Utilities|Array|Get(acopy) (Variables|Evolution|GetTracks) TrackNumber)))))

(fn StartEvaluationforIdleExecutor
  (params (Car :type Sedan%20Object%20Reference) (Genome :type Genome%20Data%20Object%20Reference))
  (Utilities|FlowControl|Sequence
    (:then_0
      ;[1 1 1] Get the Controller from the car
      (bind _astensorflow_controller (Utilities|Casting|CastToTensorflowController (AI|GetAIController Car)))
      (LocalVariables|SetTFController _astensorflow_controller))
    (:then_1
      (Physics|SetSimulatePhysics (Variables|/Script/PhysXVehicles.WheeledVehicle|GetMesh Car) false)
      (bind _selectedtrack (CallFunction|TeleportCartoStartOfTrack Car (Variables|Evolution|GettrackIdForCurrentGeneration)))
      (LocalVariables|SetTrack _selectedtrack)
      (Physics|SetSimulatePhysics (Variables|/Script/PhysXVehicles.WheeledVehicle|GetMesh Car) true))
    (:then_2
      ;[1 1 1] Set Genome Reference and start evaluation
      (Default|SetGenomeandInitialize (LocalVariables|GetTFController) Genome (LocalVariables|GetTrack))
      (Default|StartEvaluation (LocalVariables|GetTFController)))))

(fn TryEvaluateNextGenome
  (params (Car :type Sedan%20Object%20Reference))
  (bind (_hasunevaluatedgenome _genome) (Default|GetNextGenomeforEvaluation (Variables|Evolution|GetGeneticAlgorithm)))
  (if _hasunevaluatedgenome
    (CallFunction|StartEvaluationforIdleExecutor Car _genome)
    (else
      (bind _isdone (CallFunction|CheckGenerationSimulationDone))
      (if _isdone
        (CallFunction|GotoNextGeneration)))))

(fn CheckGenerationSimulationDone
  (Utilities|FlowControl|Sequence
    (:then_0
      ;[1 1 1] not all Executors done?
      (for _array_element (Variables|Evolution|GetCars)
        (bind _astensorflow_controller (Utilities|Casting|CastToTensorflowController (AI|GetAIController _array_element)))
        (if (Default|IsEvaluating _astensorflow_controller)
          (return false))))
    (:then_1
      ;[1 1 1] not all Genomes simulated?
      (bind _isdone (Default|IsGenerationCompletelySimulated (Variables|Evolution|GetGeneticAlgorithm)))
      (if (not _isdone)
        (return false)))
    (:then_2
      ;[1 1 1] All done!
      (return true))))

(fn GotoNextGeneration
  (bind _geneticalgorithm (Variables|Evolution|GetGeneticAlgorithm))
  (Default|IncrementGenerationNumber (Variables|Evolution|GetGeneticAlgorithm))
  (Class|EvaluationFunctionLibrary|WriteFitness (Variables|/Game/Blueprint/Evolution/GeneticAlgorithm.GeneticAlgorithm_C|GetPopulation _geneticalgorithm) (Variables|/Game/Blueprint/Evolution/GeneticAlgorithm.GeneticAlgorithm_C|GetGeneration _geneticalgorithm))
  (Default|Selection (Variables|Evolution|GetGeneticAlgorithm))
  (Default|MutatePopulation (Variables|Evolution|GetGeneticAlgorithm))
  (Default|SetStatetoReadyandResetFitness (Variables|Evolution|GetGeneticAlgorithm))
  (CallFunction|SelectRandomTrack)
  ;[1 1 1] start evaluation
  (for _array_element (Variables|Evolution|GetCars)
    (CallFunction|TryEvaluateNextGenome _array_element)))

(fn SelectRandomTrack
  (Variables|Evolution|SettrackIdForCurrentGeneration (Math|Random|RandomIntegerinRange 0 (- (Utilities|Array|Length (Variables|Evolution|GetTracks)) 1))))

(fn IgnoreOtherEvaluators
  (for (_array_element _array_index) (Variables|Evolution|GetCars)
    (for (_array_element_2 _array_index_2) (Variables|Evolution|GetCars)
      (if (!= _array_index_2 _array_index)
        (Default|AddCartoIgnoredActors _array_element _array_element_2)))))

(fn StopCarMovement
  (params (Car :type Sedan%20Object%20Reference))
  (Components|Movement|StopMovementImmediately (Variables|/Script/PhysXVehicles.WheeledVehicle|GetVehicleMovement Car)))