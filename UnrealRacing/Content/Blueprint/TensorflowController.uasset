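; AI controller that drives a Sedan with a TensorFlow neural network to evaluate genomes for neuroevolution.
; It sends greyscale camera pixels as JSON, waiting for each result before the next request, then applies throttle, steering and handbrake.
; Fitness is furthest progress along the track spline, ignoring large jumps.
; Track time limits end runs and request the next genome from EvolutionGM; flagged genomes mutate using one from the population's tail.
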(event OnInputResults(TensorflowComponent)
  (params (Results :type String))
  ;[1 1 1] Parse the action result of the network and execute the actions
  (Variables|Default|SetlastTickProcessed true)
  (bind _returnvalue (Class|SIOJLibrary|JsonObjecttoStruct (Class|SIOJLibrary|ToJsonObject(JsonValue) (Class|SIOJsonValue|ValuefromJsonString Results)) (Variables|Default|GetNNOutput)))
  (if _returnvalue
    (CallFunction|ExecuteNNActions)
    (else
      (Development|PrintString "NN RESULT HAS WRONG FORMAT"))))

(event Custom|MutateGenome
  (bind _populationsize (CallFunction|GetPopulationSize))
  ;[1 1 1] Call Mutate for the current genome
  (Default|CallCustomFunction (Variables|Default|GetTensorflowComponent) "mutate" (Utilities|String|ToString(Integer) (CallFunction|GetGenomeIDforPosition (Math|Random|RandomIntegerinRange (Math|Float|Truncate (* _populationsize 0.9)) (- _populationsize 1))))))

(event Custom|StartEvaluation
  ;[1 1 1] Starts the evaluation
  (Variables|Fitness|Setfitness 0.0)
  (Variables|Fitness|SetevaluationTime 0.0)
  (Variables|Fitness|SetexecuteEvaluation true)
  (Variables|Default|SetlastTickProcessed true))

(event Custom|StopEvaluation
  ;[1 1 1] Stops the evaluation
  (Variables|Fitness|SetexecuteEvaluation false)
  (Utilities|FlowControl|Sequence
    (:then_0
      (Variables|/Script/UnrealRacing.GenomeData|SetevaluationState (Variables|Default|GetGenomeRef) "Done"))
    (:then_1
      (bind _asevolution_gm (Utilities|Casting|CastToEvolutionGM (Game|GetGameMode)))
      (Default|TryEvaluateNextGenome _asevolution_gm (Variables|Default|GetCarPawn)))))

(event EventTick
  (params (DeltaSeconds :type Float%20%28single-precision%29))
  (if (and (Variables|Fitness|GetexecuteEvaluation) (Variables|Default|GetlastTickProcessed))
    (Utilities|FlowControl|Sequence
      (:then_0
        ;[1 1 1] Evaluate Network each Tick
        (CallFunction|EvaluateNeuralNetwork)
        (Variables|Default|SetlastTickProcessed false))
      (:then_1
        ;[1 1 1] Update the fitness value
        (CallFunction|UpdateFitness))
      (:then_2
        ;[1 1 1] Update execution time
        (Variables|Fitness|SetevaluationTime (+ (Variables|Fitness|GetevaluationTime) DeltaSeconds)))
      (:then_3
        ;[1 1 1] Stop Evaluation if above track time
        (if (>= (Variables|Fitness|GetevaluationTime) (Default|CalculateMaxTrackTime (Variables|Default|GetTrackRef)))
          (CallFunction|StopEvaluation))))))

(event EventOnPossess
  (params (PossessedPawn :type Pawn%20Object%20Reference))
  ;[1 1 1] Store Pawn in Variable
  (bind _assedan (Utilities|Casting|CastToSedan PossessedPawn)
    (:then
      (Variables|Default|SetCarPawn _assedan))
    (:CastFailed
      (Development|PrintString "Failed to cast to the correct car pawn!"))))

(fn ConstructionScript)

(fn EvaluateNeuralNetwork
  (bind _carpawn (Variables|Default|GetCarPawn))
  (Utilities|FlowControl|Sequence
    (:then_0
      ;[1 1 1] Create JSON Object
      (bind _returnvalue (Class|SIOJsonObject|ConstructJsonObject))
      (LocalVariables|SetRequestJSONObject _returnvalue))
    (:then_1
      ;[1 1 1] Set Data
      (bind _grayscaleimage (Default|GetGreyscaleSceneViewforAI _carpawn))
      (Class|SIOJsonObject|SetObjectField (LocalVariables|GetRequestJSONObject) "TFData" (Class|SIOJLibrary|StructtoJsonObject (Utilities|Struct|MakeTFInputData _grayscaleimage (Variables|/Game/Blueprint/Sedan/Sedan.Sedan_C|GetRenderTargetSize _carpawn)))))
    (:then_2
      ;[1 1 1] Send the Data to the Script
      (Default|SendJsonInput (Variables|Default|GetTensorflowComponent) (Class|SIOJsonObject|EncodeJson (LocalVariables|GetRequestJSONObject))))))

(fn ExecuteNNActions
  (Utilities|FlowControl|Sequence
    (:then_0
      ;[1 1 1] Throttle
      (Default|Throttle (Variables|Default|GetCarPawn) (.acceleration (Variables|Default|GetNNOutput))))
    (:then_1
      ;[1 1 1] Steering
      (Default|Steer (Variables|Default|GetCarPawn) (.right (Variables|Default|GetNNOutput))))
    (:then_2
      ;[1 1 1] Handbreak
      (Default|Handbreak (Variables|Default|GetCarPawn) (.handbreakpulled (Variables|Default|GetNNOutput))))))

(fn IsEvaluating
  (return (Variables|Fitness|GetexecuteEvaluation)))

(fn CalculateFitness
  (return (CallFunction|FindDistanceAlongSplineClosesttoWorldLocation (Transformation|GetActorLocation (Variables|Default|GetCarPawn)) (Variables|/Game/Blueprint/Road/BP_Track.BP_Track_C|GetSpline (Variables|Default|GetTrackRef)))))

(fn FindDistanceAlongSplineClosesttoWorldLocation
  (params (Location :type Vector) (Spline :type Spline%20Component%20Object%20Reference))
  (return (/ (Class|SplineComponent|FindInputKeyClosesttoWorldLocation Spline Location) (Math|Conversions|ToFloat(Integer) (- (Spline|GetNumberOfSplinePoints Spline) (Math|Conversions|ToInteger(Boolean) (not (Class|SplineComponent|IsClosedLoop Spline))))))))

(fn SetGenomeandInitialize
  (params (NextGenome :type Genome%20Data%20Object%20Reference) (NextTrack :type BP%20Track%20Object%20Reference))
  (Utilities|FlowControl|Sequence
    (:then_0
      ;[1 1 1] Set Values
      (Variables|Fitness|SetexecuteEvaluation false)
      (Variables|Default|SetTrackRef NextTrack)
      (Variables|Default|SetGenomeRef NextGenome))
    (:then_1
      ;[1 1 1] Call initialize
      (Default|CallCustomFunction (Variables|Default|GetTensorflowComponent) "initialize" (Utilities|String|ToString(Integer) (Variables|/Script/UnrealRacing.GenomeData|GetgenomeID (Variables|Default|GetGenomeRef)))))
    (:then_2
      ;[1 1 1] Call mutate if needed
      (if (Variables|/Script/UnrealRacing.GenomeData|GetshouldMutate (Variables|Default|GetGenomeRef))
        (CallFunction|MutateGenome)
        (Variables|/Script/UnrealRacing.GenomeData|SetshouldMutate (Variables|Default|GetGenomeRef) false)))))

(fn UpdateFitness
  (bind _currentfitness (CallFunction|CalculateFitness))
  (if (> _currentfitness (Variables|Fitness|Getfitness))
    (LocalVariables|SetNewFitness _currentfitness)
    ;[1 1 1] Check if the delta is whithin the threshold
    (if (<= (Math|Float|Absolute(Float) (- (LocalVariables|GetNewFitness) (Variables|/Script/UnrealRacing.GenomeData|Getfitness (Variables|Default|GetGenomeRef)))) (Variables|Fitness|GetFitnessDeltaThreshold))
      ;[1 1 1] Set if within threshold
      (Variables|/Script/UnrealRacing.GenomeData|Setfitness (Variables|Default|GetGenomeRef) (LocalVariables|GetNewFitness)))))

(fn GetPopulationSize
  (bind _asevolution_gm (Utilities|Casting|CastToEvolutionGM (Game|GetGameMode))
    (:then
      (return (Variables|/Game/Blueprint/Evolution/GeneticAlgorithm.GeneticAlgorithm_C|GetPopulationSize (Variables|/Game/Blueprint/EvolutionGM.EvolutionGM_C|GetGeneticAlgorithm _asevolution_gm))))
    (:CastFailed
      (Development|PrintString "Invalid Gamemode")
      (return -1))))

(fn GetGenomeIDforPosition
  (params (Index :type Integer))
  (bind _asevolution_gm (Utilities|Casting|CastToEvolutionGM (Game|GetGameMode)))
  (return (Variables|/Script/UnrealRacing.GenomeData|GetgenomeID (Utilities|Array|Get(acopy) (Variables|/Game/Blueprint/Evolution/GeneticAlgorithm.GeneticAlgorithm_C|GetPopulation (Variables|/Game/Blueprint/EvolutionGM.EvolutionGM_C|GetGeneticAlgorithm _asevolution_gm)) Index))))